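; Actor that opens a file dialog on BeginPlay and imports the chosen 3D model files at runtime through Assimp.
; UseAsync selects async or blocking import, with async progress callbacks feeding the same per-scene build logic.
; Each scene's materials become dynamic instances with embedded diffuse and normal textures, appended to a shared Materials array.
; Each mesh spawns an actor with a rotated procedural mesh component, its material picked from that array by index.
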(event `self.ReceiveBeginPlay`
  (bind _returnvalue (`AssimpFunctionLibrary.ProcessPreset_TargetRealtime_Quality`))
  (bind _returnvalue_2 (`GameplayStatics.GetGameMode`))
  (bind _outfilenames (`AssimpFunctionLibrary.OpenFileDialogue` ""))
  (if (`self.Use Async`)
    (`AssimpFunctionLibrary.ImportScenesAsync` "/Script/UE_Assimp.Default__AssimpFunctionLibrary" _outfilenames _returnvalue_2 _returnvalue false (delegate `CustomEvent_0`) (delegate `CustomEvent_2`))
    (else
      (bind _scenes (`AssimpFunctionLibrary.ImportScenes` _outfilenames _returnvalue_2 _returnvalue))
      (for _array_element _scenes
        (`|ExecutionSequence` :!label _label
          (:`then_0`
            (bind _returnvalue_3 (select `bool` (`self.Use Async`) :`false` _array_element :`true` (stale `CustomEvent_0` ImportedScene)))
            (for _array_element_2 (`AIScene.GetAllMaterials` _returnvalue_3)
              (bind _returnvalue_4 (`KismetMaterialLibrary.CreateDynamicMaterialInstance` null "None" "Transient"))
              (`KismetArrayLibrary.Array_Add` (`self.Materials`) _returnvalue_4)
              (`MaterialInstanceDynamic.SetTextureParameterValue` _returnvalue_4 "BaseColor" (`AIScene.GetEmbeddedTexture` _returnvalue_3 (`.Path` (`AIMaterial.GetMaterialTexture` _array_element_2 "AiTextureType_DIFFUSE" 0 "AiTextureMapping_UV")) false))
              (`MaterialInstanceDynamic.SetTextureParameterValue` _returnvalue_4 "Normal" (`AIScene.GetEmbeddedTexture` _returnvalue_3 (`.Path` (`AIMaterial.GetMaterialTexture` _array_element_2 "AiTextureType_NORMALS" 0 "AiTextureMapping_UV")) true))
              (`KismetSystemLibrary.PrintString` "Set Texture reached")))
          (:`then_1`
            (for _array_element_3 (`AIScene.GetAllMeshes` _returnvalue_3)
              (bind (_vertices _triangles _normals _uv0 _tangents) (`AIMesh.GetMeshDataForProceduralMesh` _array_element_3))
              (bind _returnvalue_5 (`|SpawnActorFromClass` "/Script/Engine.Actor" (`KismetMathLibrary.MakeTransform` (0.0 0.0 200.0)) "AlwaysSpawn" "SelectDefaultAtRuntime" null null))
              (bind _returnvalue_6 (`AddComponent|NODE_AddProceduralMeshComponent-0` :`self` _returnvalue_5 :`RelativeTransform` (`KismetMathLibrary.MakeTransform` (0.0 0.0 0.0) (struct :`Pitch` -90.0 :`Yaw` -90.0))))
              (`ProceduralMeshComponent.CreateMeshSection_LinearColor` :`self` _returnvalue_6 :`Vertices` _vertices :`Triangles` _triangles :`Normals` _normals :`UV0` _uv0 :`Tangents` _tangents)
              (`PrimitiveComponent.SetMaterial` _returnvalue_6 0 (`|GetArrayItem` (`self.Materials`) (`AIMesh.GetMaterialIndex` _array_element_3)))
              (`KismetSystemLibrary.PrintString` "Reached end Node"))))))))

(event `CustomEvent_0`
  (params (NormalPercentage :type "Float (single-precision)") (ImportedScene :type "AIScene Object Reference"))
  (goto _label))

(event `CustomEvent_2`
  (params (ImportedScenes :type "Array of AIScene Object Reference (by ref)"))
  (`KismetSystemLibrary.PrintString` "Hello"))

(fn `UserConstructionScript`)