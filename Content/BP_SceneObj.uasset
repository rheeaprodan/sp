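; BP_SceneObj is a Blueprint that creates a new numbered scene level and opens it.
; NewScene uses AssetTools to duplicate an asset into /Game/ under a name built from the incremented counter, then opens it by name and returns that name.
; An unconnected older path streams EmptyScene as a named level instance and records it in a map.
; The event graph and construction script are empty.
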(fn `NewScene`
  (params (Counter :type Integer64))
  (returns (Scene :type Name))
  (bind _returnvalue (`AssetToolsHelpers.GetAssetTools`))
  (bind _returnvalue_2 (`AssetTools.DuplicateAsset` _returnvalue (`KismetTextLibrary.Conv_TextToString` (`|FormatText` "Scene{Counter}" (+ Counter 1))) "/Game/" null))
  (bind _returnvalue_3 (`KismetStringLibrary.Conv_StringToName` (`KismetSystemLibrary.GetObjectName` _returnvalue_2)))
  (`GameplayStatics.OpenLevel` _returnvalue_3)
  (return _returnvalue_3))

(fn `UserConstructionScript`)